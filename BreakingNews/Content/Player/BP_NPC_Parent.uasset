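; BP_NPC_Parent is an NPC Blueprint, named as a parent class, for a vehicle driven by throttle and steering.
; On BeginPlay it initializes all systems and sets full engine throttle, with no active steering and an empty Tick.
; A disconnected chase graph steers toward the player's position plus velocity and scales throttle by how directly the NPC faces the player, but it never runs.
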(event `self.ReceiveBeginPlay`
  (`self.InitializeAllSystems`)
  (`self.SetEngineThrottle` 1.0))

(event `self.ReceiveTick`
  (params (DeltaSeconds :type "Float (single-precision)")))

(fn `UserConstructionScript`)