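; Parent player vehicle for a car-chase game, with manual throttle and handbrake and lane-based automatic steering.
; Steering input steps between six lanes on a short cooldown, picking a spline from the road manager.
; Each tick it steers toward a look-ahead point on that spline, flipping the look-ahead direction for the upper three lanes.
; News-ticker distance score and crash-restart logic are present but disconnected.
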(event `self.ReceiveBeginPlay`
  (`self.InitializeAllSystems`)
  (`PlayerController.ClientStartCameraShake` :`self` (`GameplayStatics.GetPlayerController` 0) :`Shake` "/Game/Player/CS_Chase.CS_Chase_C"))

(event `InputAxis|Throttle`
  (params (AxisValue :type "Float (single-precision)"))
  (`self.SetEngineThrottle` (`KismetMathLibrary.FClamp` AxisValue -1.0)))

(event `InputAxis|Steering`
  (params (AxisValue :type "Float (single-precision)"))
  (bind _lane (`self.Lane`))
  (if (> (`KismetMathLibrary.Abs` AxisValue) 0.1)
    (if (`self.bCanChangeLane`)
      (set `self.Lane` (`KismetMathLibrary.Clamp` (- (`self.Lane`) (`KismetMathLibrary.FTrunc` (`KismetMathLibrary.SignOfFloat` AxisValue))) 0 5))
      (set `self.bCanChangeLane` false)
      (set `self.LaneSpline_Ref` (`|GetArrayItem` (`/Game/LevelGeneration/BP_RandomWorldGenerator.LaneArray` (`self.RoadManager_Ref`)) _lane))
      (`KismetSystemLibrary.PrintString` (`KismetStringLibrary.Conv_IntToString` _lane))
      (`KismetSystemLibrary.Delay` 0.2)
      (set `self.bCanChangeLane` true))))

(event `Steering`
  (params (DeltaSeconds :type "Float (double-precision)"))
  (bind _returnvalue (`self.K2_GetActorLocation`))
  (bind _returnvalue_2 (`SplineComponent.FindLocationClosestToWorldLocation` (`self.LaneSpline_Ref`) (+ _returnvalue (* (`SplineComponent.FindDirectionClosestToWorldLocation` (`self.LaneSpline_Ref`) (`self.K2_GetActorLocation`) "World") (* 3000.0 (`KismetMathLibrary.SelectFloat` 1.0 -1.0 (<= (`self.Lane`) 2))))) "World"))
  (set `self.Target` _returnvalue_2)
  (`self.SetSteering` (`KismetMathLibrary.Dot_VectorVector` (`KismetMathLibrary.Conv_RotatorToVector` (`KismetMathLibrary.FindLookAtRotation` _returnvalue _returnvalue_2)) (`self.GetActorRightVector`))))

(event `InputAction|Handbrake`
  (params (Key :type "Key Structure"))
  (:`Pressed`
    (`self.SetHandbrake` true))
  (:`Released`
    (`self.SetHandbrake` false)))

(event `self.StaticMesh.OnComponentHit`
  (params (HitComponent :type "PrimitiveComponent Object Reference") (OtherActor :type "Actor Object Reference") (OtherComp :type "PrimitiveComponent Object Reference") (NormalImpulse :type "Vector Structure") (Hit :type "HitResult Structure (by ref)")))

(event `self.ReceiveTick`
  (params (DeltaSeconds :type "Float (single-precision)"))
  (`self.Steering` DeltaSeconds))

(fn `UserConstructionScript`)