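; Player truck Blueprint that attaches a separately spawned wheel actor to its body through physics.
; On BeginPlay it spawns a MultiWheel1 actor at the PhysicsConstraint component's world transform, ignoring collisions.
; It then binds the truck's StaticMesh to the spawned actor's StaticMesh with that constraint at runtime.
; Tick, overlap and the construction script add no logic of their own.
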(event `self.ReceiveBeginPlay`
  (`parent.ReceiveBeginPlay`)
  (bind _returnvalue (`|SpawnActorFromClass` "/Game/Player/MultiWheel1.MultiWheel1_C" (`SceneComponent.K2_GetComponentToWorld` (`self.PhysicsConstraint`)) "AlwaysSpawn" "OverrideRootScale" null null))
  (`PhysicsConstraintComponent.SetConstrainedComponents` (`self.PhysicsConstraint`) (`self.StaticMesh`) "None" (`/Game/Player/MultiWheel1.StaticMesh` _returnvalue) "None"))

(fn `UserConstructionScript`
  (`parent.UserConstructionScript`))