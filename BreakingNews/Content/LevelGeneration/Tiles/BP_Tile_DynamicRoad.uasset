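; Road tile Blueprint for level generation with a helper that places a building on each side of the road.
; CreateIntersectionBuildings adds two static mesh components, offsets them along ±Y by building and root bounds, and mirrors the +Y one via negative scale.
; GetRandomBuilding is called separately for mesh and offset, and its random array pick appears unconnected.
; BeginPlay and construction only call the parent; nothing here calls the helper.
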(event `self.ReceiveBeginPlay`
  (`parent.ReceiveBeginPlay`))

(fn `CreateIntersectionBuildings`
  (params (InputRoadBuildingsArray :type "Array of StaticMesh Object Reference") (RootStaticMeshComponent :type "StaticMeshComponent Object Reference"))
  (locals (LInputRoadBuildingsArray :type "Array of StaticMesh Object Reference") (LRootStaticMeshComponent :type "StaticMeshComponent Object Reference"))
  (bind _randomstaticmesh (`self.GetRandomBuilding` (`local.LInputRoadBuildingsArray`)))
  (set `local.LInputRoadBuildingsArray` InputRoadBuildingsArray)
  (set `local.LRootStaticMeshComponent` RootStaticMeshComponent)
  ;[1 1 1] Top building
  (bind _returnvalue (`AddComponent|NODE_AddStaticMeshComponent-2`))
  (`StaticMeshComponent.SetStaticMesh` _returnvalue _randomstaticmesh)
  (`SceneComponent.K2_SetRelativeTransform` _returnvalue (`KismetMathLibrary.MakeTransform` (`KismetMathLibrary.MakeVector` 0.0 (+ (.y (`.BoxExtent` (`KismetMathLibrary.BreakBoxSphereBounds` (`StaticMesh.GetBounds` _randomstaticmesh)))) (.y (`.BoxExtent` (`KismetSystemLibrary.GetComponentBounds` (`local.LRootStaticMeshComponent`)))))) (struct) (1.0 -1.0 1.0)) false false)
  ;[1 1 1] Bottom right building
  (bind _returnvalue_2 (`AddComponent|NODE_AddStaticMeshComponent-3`))
  (`StaticMeshComponent.SetStaticMesh` _returnvalue_2 (`self.GetRandomBuilding` (`local.LInputRoadBuildingsArray`)))
  (`SceneComponent.K2_SetRelativeTransform` _returnvalue_2 (`KismetMathLibrary.MakeTransform` (`KismetMathLibrary.MakeVector` 0.0 (* (+ (.y (`.BoxExtent` (`KismetMathLibrary.BreakBoxSphereBounds` (`StaticMesh.GetBounds` (`self.GetRandomBuilding` (`local.LInputRoadBuildingsArray`)))))) (.y (`.BoxExtent` (`KismetSystemLibrary.GetComponentBounds` (`local.LRootStaticMeshComponent`))))) -1.0))) false false))

(fn `UserConstructionScript`
  (`parent.UserConstructionScript`))