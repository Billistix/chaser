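; Level generation tile for a 150m dynamic road that dresses itself with randomly chosen buildings.
; On BeginPlay, after the parent logic, CreateIntersectionBuildings adds two static mesh components at runtime, offset equally on opposite sides along the local Y axis.
; Each gets its mesh through GetRandomBuilding from the RoadBuildings array.
; The negative-Y building uses a negative Y scale to mirror it toward the opposite side.
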(event `self.ReceiveBeginPlay`
  (`parent.ReceiveBeginPlay`)
  (`self.CreateIntersectionBuildings`))

(fn `CreateIntersectionBuildings`
  ;[1 1 1] Top building
  (bind _returnvalue (`AddComponent|NODE_AddStaticMeshComponent-2`))
  (`StaticMeshComponent.SetStaticMesh` _returnvalue (`self.GetRandomBuilding` (`self.RoadBuildings`)))
  (`SceneComponent.K2_SetRelativeTransform` _returnvalue (`KismetMathLibrary.MakeTransform` (0.0 4310.0 0.0) (struct) (1.0 1.0 1.0)) false false)
  ;[1 1 1] Bottom right building
  (bind _returnvalue_2 (`AddComponent|NODE_AddStaticMeshComponent-3`))
  (`StaticMeshComponent.SetStaticMesh` _returnvalue_2 (`self.GetRandomBuilding` (`self.RoadBuildings`)))
  (`SceneComponent.K2_SetRelativeTransform` _returnvalue_2 (`KismetMathLibrary.MakeTransform` (0.0 -4310.0 0.0) (struct) (1.0 -1.0 1.0)) false false))

(fn `UserConstructionScript`
  (`parent.UserConstructionScript`))