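; Intersection tile for level generation that adds four corner buildings when play begins.
; CreateIntersectionBuildings adds a static mesh component at each corner, with its mesh requested from GetRandomBuilding using the IntersectionBuildings array.
; Negative scale or a 180-degree rotation orients each corner, so one set of meshes serves all four.
; The random-index lookup inside GetRandomBuilding appears as unused, with no connected return.
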(event `self.ReceiveBeginPlay`
  (`parent.ReceiveBeginPlay`)
  (`self.CreateIntersectionBuildings`))

(fn `CreateIntersectionBuildings`
  ;[1 1 1] Top right building
  (bind _returnvalue (`AddComponent|NODE_AddStaticMeshComponent-2`))
  (`StaticMeshComponent.SetStaticMesh` _returnvalue (`self.GetRandomBuilding` (`self.IntersectionBuildings`)))
  (`SceneComponent.K2_SetRelativeTransform` _returnvalue (`KismetMathLibrary.MakeTransform` (4400.0 -4750.0 0.0)) false false)
  ;[1 1 1] Bottom right building
  (bind _returnvalue_2 (`AddComponent|NODE_AddStaticMeshComponent-3`))
  (`StaticMeshComponent.SetStaticMesh` _returnvalue_2 (`self.GetRandomBuilding` (`self.IntersectionBuildings`)))
  (`SceneComponent.K2_SetRelativeTransform` _returnvalue_2 (`KismetMathLibrary.MakeTransform` (4400.0 4750.0 0.0) (struct) (1.0 -1.0 1.0)) false false)
  ;[1 1 1] Bottom left building
  (bind _returnvalue_3 (`AddComponent|NODE_AddStaticMeshComponent-4`))
  (`StaticMeshComponent.SetStaticMesh` _returnvalue_3 (`self.GetRandomBuilding` (`self.IntersectionBuildings`)))
  (`SceneComponent.K2_SetRelativeTransform` _returnvalue_3 (`KismetMathLibrary.MakeTransform` (-4400.0 4750.0 0.0) (struct :`Yaw` 180.0)) false false)
  ;[1 1 1] Top left building
  (bind _returnvalue_4 (`AddComponent|NODE_AddStaticMeshComponent-5`))
  (`StaticMeshComponent.SetStaticMesh` _returnvalue_4 (`self.GetRandomBuilding` (`self.IntersectionBuildings`)))
  (`SceneComponent.K2_SetRelativeTransform` _returnvalue_4 (`KismetMathLibrary.MakeTransform` (-4400.0 -4750.0 0.0) (struct) (-1.0 1.0 1.0)) false false))

(fn `UserConstructionScript`
  (`parent.UserConstructionScript`))