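; BP_Savegame is a save game object holding level, player position, control rotation and play time.
; Manual saves require BPI_SavableCharacter on the player, update play time since load, then write the slot.
; Quicksave reuses this with a fixed slot name.
; Creation setup, timestamped autosaves with pruning and scene-capture thumbnails are disconnected, so those entry points do nothing; screenshot loading is also empty.
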(event `OnCreate`
  ;[1 1 1] initialize timestamps
)

(event `OnLoad`
  ;[1 1 1] init load time
  (set `self.LoadedOn` (`KismetMathLibrary.Now`)))

(fn `FormatDate`
  (params (Format :type String) (DateTime :type "DateTime Structure"))
  (returns (FormatedDate :type String))
  (bind (_year _month _day _hour _minute _second) (`KismetMathLibrary.BreakDateTime` DateTime))
  (`KismetStringLibrary.ReplaceInline` Format "%y" (`self.FormatInt00` _year) "CaseSensitive")
  (`KismetStringLibrary.ReplaceInline` Format "%m" (`self.FormatInt00` _month) "CaseSensitive")
  (`KismetStringLibrary.ReplaceInline` Format "%d" (`self.FormatInt00` _day) "CaseSensitive")
  (`KismetStringLibrary.ReplaceInline` Format "%H" (`self.FormatInt00` _hour) "CaseSensitive")
  (`KismetStringLibrary.ReplaceInline` Format "%M" (`self.FormatInt00` _minute) "CaseSensitive")
  (`KismetStringLibrary.ReplaceInline` Format "%S" (`self.FormatInt00` _second) "CaseSensitive")
  (return Format))

(fn `FormatInt00`
  (params (Int :type Integer))
  (returns (String :type String))
  (bind _returnvalue (`KismetStringLibrary.Conv_IntToString` Int))
  (return (select `bool` (<= Int 9) :`false` _returnvalue :`true` (`KismetStringLibrary.Concat_StrStr` "0" _returnvalue))))

(fn `GetSaveDisplayName`
  (returns (DisplayName :type String))
  ;[1 1 1] override thsi function, if you want to specify a custom save name
  (return ""))

(fn `LoadScreenshot`
  (returns (` Screenshot` :type "Texture2D Object Reference")))

(fn `SaveAsAutosave`
  (params (Level :type String) (Player :type "Character Object Reference") (Controller :type "PlayerController Object Reference"))
  (locals (AutoSaveSlots :type "Array of String"))
  ;[1 1 1] create new save
)

(fn `SaveAsManualSave`
  (params (SlotName :type String) (Level :type String) (Player :type "Character Object Reference") (Controller :type "PlayerController Object Reference"))
  (locals (Slot :type String))
  (bind _returnvalue (`KismetMathLibrary.Now`))
  ;[1 1 1] set save data
  (set `local.Slot` SlotName)
  (set `self.Level` Level)
  (set `self.PlayerPosition` (`Actor.K2_GetActorLocation` Player))
  (set `self.PlayerRotation` (`Controller.GetControlRotation` Controller))
  ;[1 1 1] Screenshot and interface interaction
  (if (`KismetSystemLibrary.DoesImplementInterface` Player "/Game/UserInterface/Blueprints/SaveSelection/BPI_SavableCharacter.BPI_SavableCharacter_C")
    (bind _scenecapturecomponent (message `/Game/UserInterface/Blueprints/SaveSelection/BPI_SavableCharacter.GetSceneCaptureComponent2D` Player))
    (`self.TakeScreenshot` _scenecapturecomponent)
    ;[1 1 1] update time played
    (set `self.TotalTimePlayed` (+ (`self.TotalTimePlayed`) (- _returnvalue (`self.LoadedOn`))))
    (set `self.LoadedOn` _returnvalue)
    ;[1 1 1] save it
    (`GameplayStatics.SaveGameToSlot` self (`local.Slot`))
    (else
      (`KismetSystemLibrary.PrintString` Player "Your character has to implement the interface BPI_SavableCharacter!" true true (struct :`R` 0.58 :`A` 1.0) 10.0))))

(fn `SaveAsQuicksave`
  (params (Level :type String) (Player :type "Character Object Reference") (Controller :type "PlayerController Object Reference"))
  (`self.SaveAsManualSave` "Quicksave" Level Player Controller))

(fn `TakeScreenshot`
  (params (SceneCaptureComponent2D :type "SceneCaptureComponent2D Object Reference (by ref)")))