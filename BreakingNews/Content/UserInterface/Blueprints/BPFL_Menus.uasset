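; Blueprint function library of menu UI helpers for notifications, FPS counter display and date/time text.
; ShowNotification and GetFPSCounter reuse the first existing widget of their class or create one at a high viewport Z-order.
; ShowFps and ToggleFps switch the counter between hit-test-invisible and collapsed, with alignment applied only on creation.
; FormatDateTime substitutes strftime-like tokens in a pattern, zero-padding values through FormatInt00.
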(fn `FormatDateTime`
  (params (Pattern :type String) (DateTime :type "DateTime Structure"))
  (returns (FormatedString :type String))
  (bind (_year _month _day _hour _minute _second) (`KismetMathLibrary.BreakDateTime` DateTime))
  (`KismetStringLibrary.ReplaceInline` Pattern "%y" (`self.FormatInt_00` _year) "CaseSensitive")
  (`KismetStringLibrary.ReplaceInline` Pattern "%m" (`self.FormatInt_00` _month) "CaseSensitive")
  (`KismetStringLibrary.ReplaceInline` Pattern "%d" (`self.FormatInt_00` _day) "CaseSensitive")
  (`KismetStringLibrary.ReplaceInline` Pattern "%H" (`self.FormatInt_00` _hour) "CaseSensitive")
  (`KismetStringLibrary.ReplaceInline` Pattern "%M" (`self.FormatInt_00` _minute) "CaseSensitive")
  (`KismetStringLibrary.ReplaceInline` Pattern "%S" (`self.FormatInt_00` _second) "CaseSensitive")
  (return Pattern))

(fn `FormatInt_00`
  (params (Number :type Integer))
  (returns (Formated :type String))
  (bind _returnvalue (`KismetStringLibrary.Conv_IntToString` Number))
  (return (select `bool` (<= Number 9) :`false` _returnvalue :`true` (`KismetStringLibrary.Concat_StrStr` "0" _returnvalue))))

(fn `GetFPSCounter`
  (params (OwningPlayer :type "PlayerController Object Reference") (HorizontalAlignment :type "EHorizontalAlignment Enum" :default "HAlign_Fill") (VerticalAlignment :type "EVerticalAlignment Enum" :default "VAlign_Fill"))
  (returns (Widget :type "/Game/UserInterface/Widgets/Generics/WBP_FpsCounter Object Reference"))
  (bind _foundwidgets (`WidgetBlueprintLibrary.GetAllWidgetsOfClass` OwningPlayer "/Game/UserInterface/Widgets/Generics/WBP_FpsCounter.WBP_FpsCounter_C" false))
  (if (== (`KismetArrayLibrary.Array_Length` _foundwidgets) 0)
    (bind _returnvalue (`|CreateWidget` "/Game/UserInterface/Widgets/Generics/WBP_FpsCounter.WBP_FpsCounter_C" OwningPlayer HorizontalAlignment VerticalAlignment))
    (`Widget.SetVisibility` _returnvalue "Collapsed")
    (`UserWidget.AddToViewport` _returnvalue 1000)
    (return _returnvalue)
    (else
      (return (`|GetArrayItem` _foundwidgets)))))

(fn `ShowFps`
  (params (OwningPlayer :type "PlayerController Object Reference") (Show :type Boolean) (HorizontalAlignment :type "EHorizontalAlignment Enum" :default "HAlign_Fill") (VerticalAlignment :type "EVerticalAlignment Enum" :default "VAlign_Fill"))
  (bind _widget (`self.GetFPSCounter` OwningPlayer HorizontalAlignment VerticalAlignment OwningPlayer))
  (`Widget.SetVisibility` _widget (select `bool` Show :`false` "Collapsed" :`true` "HitTestInvisible" :!type "ESlateVisibility Enum")))

(fn `ShowNotification`
  (params (OwningPlayer :type "PlayerController Object Reference") (NotificationText :type Text))
  (returns (NotificationPanel :type "/Game/UserInterface/Widgets/Generics/WBP_Notification Object Reference"))
  ;[1 1 1] find reference to the notification panel widget, if no reference was found, create the panel
  (bind _foundwidgets (`WidgetBlueprintLibrary.GetAllWidgetsOfClass` OwningPlayer "/Game/UserInterface/Widgets/Generics/WBP_NotificationPanel.WBP_NotificationPanel_C" false))
  (if (== (`KismetArrayLibrary.Array_Length` _foundwidgets) 0)
    (bind _returnvalue (`|CreateWidget` "/Game/UserInterface/Widgets/Generics/WBP_NotificationPanel.WBP_NotificationPanel_C" OwningPlayer))
    (`UserWidget.AddToViewport` _returnvalue 1000)
    (bind _notificationpanel (`/Game/UserInterface/Widgets/Generics/WBP_NotificationPanel.AddNotification` _returnvalue NotificationText))
    (return _notificationpanel)
    (else
      (bind _notificationpanel_2 (`/Game/UserInterface/Widgets/Generics/WBP_NotificationPanel.AddNotification` (`|GetArrayItem` _foundwidgets) NotificationText))
      (return _notificationpanel_2))))

(fn `ToggleFps`
  (params (OwningPlayer :type "PlayerController Object Reference") (HorizontalAlignment :type "EHorizontalAlignment Enum" :default "HAlign_Fill") (VerticalAlignment :type "EVerticalAlignment Enum" :default "VAlign_Fill"))
  (bind _widget (`self.GetFPSCounter` OwningPlayer HorizontalAlignment VerticalAlignment OwningPlayer))
  (`self.ShowFps` OwningPlayer (`|EnumEquality` (`Widget.GetVisibility` _widget) "Collapsed") HorizontalAlignment VerticalAlignment OwningPlayer))